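; BP_Toad is a player-controlled Paper2D flipbook character, using robot animations, that moves horizontally within fixed X bounds.
; Left and Right keys set Direction, which Tick uses to move, tilt the capsule, flip the sprite and pick idle or moving flipbooks.
; Space triggers a timeline-driven, swept dash along Direction.
; An unconnected hit sequence would add score via GI_Game, play a hit animation and temporarily reduce speed and dash force.
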(event `self.ReceiveBeginPlay`)

(event `self.ReceiveActorBeginOverlap`
  (params (OtherActor :type "Actor Object Reference")))

(event `self.ReceiveTick`
  (params (DeltaSeconds :type "Float (single-precision)"))
  (bind (_returnvalue_x _returnvalue_y _returnvalue_z) (`KismetMathLibrary.BreakVector` (`self.K2_GetActorLocation`)))
  (bind (_relativerotation_roll _relativerotation_pitch _relativerotation_yaw) (`KismetMathLibrary.BreakRotator` (`SceneComponent.RelativeRotation` (`self.CapsuleComponent`))))
  (`self.K2_SetActorLocation` (`KismetMathLibrary.MakeVector` (`KismetMathLibrary.FClamp` (+ (* DeltaSeconds (`self.VelX`) (`self.direction`)) _returnvalue_x) -50.0 1250.0) _returnvalue_y _returnvalue_z))
  (`SceneComponent.K2_SetRelativeRotation` (`self.CapsuleComponent`) (`KismetMathLibrary.RInterpTo` (`SceneComponent.RelativeRotation` (`self.CapsuleComponent`)) (`KismetMathLibrary.MakeRotator` _relativerotation_roll (* (`self.direction`) -20.0) _relativerotation_yaw) (`GameplayStatics.GetWorldDeltaSeconds`) 10.0) false false)
  (if (== (`self.direction`) -1)
    (`SceneComponent.SetRelativeScale3D` (`self.Sprite`) (-1.4 1.4 1.4))
    (elif (not (`self.sens`))
      (`SceneComponent.SetRelativeScale3D` (`self.Sprite`) (1.4 1.4 1.4))))
  (if (`self.isHurting`)
    _
    (elif (== (`self.direction`) 0)
      (`PaperFlipbookComponent.SetFlipbook` (`self.Sprite`) "/Game/image/Robots_Anims/Idle/FS_Robot_Idle.FS_Robot_Idle")
      (else
        (`PaperFlipbookComponent.SetFlipbook` (`self.Sprite`) "/Game/image/Robots_Anims/Move/FS_Robot_Moves.FS_Robot_Moves")))))

(event `Key|Left`
  (params (Key :type "Key Structure"))
  (bind _direction (`self.direction`))
  (:`Pressed`
    (set `self.direction` (+ _direction 1))
    (set `self.sens` false))
  (:`Released`
    (set `self.direction` (+ _direction -1))))

(event `Key|Right`
  (params (Key :type "Key Structure"))
  (bind _direction (`self.direction`))
  (:`Pressed`
    (set `self.direction` (+ _direction -1))
    (set `self.sens` true))
  (:`Released`
    (set `self.direction` (+ _direction 1))))

(event `Key|SpaceBar`
  (params (Key :type "Key Structure"))
  (:`Pressed`
    (`self.DashEvent`)))

(event `DashEvent`
  (bind (_relativelocation_x _relativelocation_y _relativelocation_z) (`KismetMathLibrary.BreakVector` (`SceneComponent.RelativeLocation` (`self.CapsuleComponent`))))
  (bind _output_get (set `self.StartDash` _relativelocation_x))
  (set `self.endDash` (+ _output_get (* (`self.direction`) (`self.forceDash`))))
  (bind (_direction _alpha) (`Timeline|TL_Dash` :!via `PlayFromStart`)
    (:`Update`
      (`SceneComponent.K2_SetRelativeLocation` (`self.CapsuleComponent`) (`KismetMathLibrary.MakeVector` (`KismetMathLibrary.Lerp` (`self.StartDash`) (`self.endDash`) _alpha) _relativelocation_y _relativelocation_z) true false))))

(fn `UserConstructionScript`)